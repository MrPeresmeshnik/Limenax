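; Paper2D side-scrolling player character with horizontal movement, jump via key or touch, an attack animation, timed overhead text and a health bar widget.
; Input, falling velocity and landing set CharacterStates, which UpdateAnimation maps to flipbooks, refreshed from the MoveRight axis event.
; Attack disables input for the flipbook's remaining time, while Backspace drains health until the Dead state.
; Tick pins the comment text's rotation as control yaw flips with direction.
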(event `self.ReceiveBeginPlay`
  ;[1 1 1] initialize
  (`|ExecutionSequence`
    (:`then_0`
      (`ActorComponent.SetIsReplicated` (`self.Sprite`) true))
    (:`then_1`
      (bind _returnvalue (`|CreateWidget` "/Game/Limenax/interface/Health_Bar.Health_Bar_C" (`GameplayStatics.GetPlayerController` 0)))
      (bind _output_get (set `self.Health Bar` _returnvalue))
      (`UserWidget.AddToViewport` _output_get 0))))

(event `Key|BackSpace`
  (params (Key :type "Key Structure" :default "AnyKey"))
  (:`Pressed`
    (bind _output_get (set `self.Health` (- (`self.Health`) 0.1)))
    (if (<= _output_get 0.0)
      (set `self.Character_states` "NewEnumerator4")
      (`self.DisableInput` (`GameplayStatics.GetPlayerController` 0))
      (`PaperFlipbookComponent.SetLooping` (`self.Sprite`) false))))

(event `UpdateAnimation`
  (bind _sprite (`self.Sprite`))
  (bind _sprite_2 (`self.Sprite`))
  ;[1 1 1] Handle Animation
  (switch `/Game/Limenax/Blueprints/Character_states` (`self.Character_states`)
    (:`NewEnumerator0`
      (`PaperFlipbookComponent.SetFlipbook` _sprite_2 (select `bool` (> (`KismetMathLibrary.VSize` (`self.GetVelocity`)) 0.0) :`false` "/Game/Limenax/Character/Mami_Tomoe/Mami_Tomoe_Stay.Mami_Tomoe_Stay" :`true` "/Game/Limenax/Character/Mami_Tomoe/Mami_Tomoe_run.Mami_Tomoe_run" :!type "PaperFlipbook Object Reference") :!label _label))
    (:`NewEnumerator1`
      (goto _label))
    (:`NewEnumerator2`
      (`PaperFlipbookComponent.SetFlipbook` _sprite_2 "/Game/Limenax/Character/Mami_Tomoe/Mami_Tomoe_jump.Mami_Tomoe_jump"))
    (:`NewEnumerator4`
      (`PaperFlipbookComponent.SetFlipbook` _sprite "/Game/Limenax/Character/Mami_Tomoe/Mami_Tomoe__Dead.Mami_Tomoe__Dead"))
    (:`NewEnumerator6`
      (`PaperFlipbookComponent.SetFlipbook` _sprite "/Game/Limenax/Character/Mami_Tomoe/Mami_Tomoe_A.Mami_Tomoe_A"))
    (:`NewEnumerator8`
      (`PaperFlipbookComponent.SetFlipbook` _sprite "/Game/Limenax/Character/Mami_Tomoe/Mami_Tomoe_falling.Mami_Tomoe_falling"))))

(event `InputAxis|MoveRight`
  (params (AxisValue :type "Float (single-precision)"))
  (bind (_returnvalue_x _returnvalue_y _returnvalue_z) (`KismetMathLibrary.BreakVector` (`self.GetVelocity`)))
  ;[1 1 1] Handle movement
  (`self.AddMovementInput` (1.0 0.0 0.0) AxisValue)
  ;[1 1 1] Falling
  (`/Engine/EditorBlueprintResources/StandardMacros.CompareFloat` _returnvalue_z
    (:`>`
      _)
    (:`==`
      _)
    (:`<`
      (`PaperFlipbookComponent.SetLooping` (`self.Sprite`) true)
      (set `self.Character_states` "NewEnumerator8")))
  (`self.UpdateAnimation`)
  (`/Engine/EditorBlueprintResources/StandardMacros.CompareFloat` AxisValue
    (:`>`
      (`Controller.SetControlRotation` (`self.GetController`) (`KismetMathLibrary.MakeRotator` 0.0 0.0 0.0)))
    (:`<`
      (`Controller.SetControlRotation` (`self.GetController`) (`KismetMathLibrary.MakeRotator` 0.0 0.0 180.0)))))

(event `InputAction|Jump`
  (params (Key :type "Key Structure" :default "AnyKey"))
  ;[1 1 1] Handle Jump
  (:`Pressed`
    (`self.Jump` :!label _label_2)
    (set `self.Character_states` "NewEnumerator2")
    (`self.UpdateAnimation`)
    (`PaperFlipbookComponent.SetLooping` (`self.Sprite`) false))
  (:`Released`
    (`self.StopJumping` :!label _label_3)))

(event `InputTouch`
  (params (Location :type "Vector Structure") (FingerIndex :type "ETouchIndex Enum"))
  ;[1 1 1] Handle Jump
  (:`Pressed`
    (goto _label_2))
  (:`Released`
    (goto _label_3)))

(event `self.OnLanded`
  (params (Hit :type "HitResult Structure (by ref)"))
  (`PaperFlipbookComponent.SetLooping` (`self.Sprite`) true)
  (set `self.Character_states` "NewEnumerator1"))

(event `Comment`
  (params (Text :type String))
  (bind _comments (`self.Comments`))
  (bind (_returnvalue_x _returnvalue_y _returnvalue_z) (`KismetMathLibrary.BreakVector` (`SceneComponent.K2_GetComponentLocation` (`self.CapsuleComponent`))))
  ;[1 1 1] Comment_Event
  (`TextRenderComponent.K2_SetText` _comments (`KismetTextLibrary.Conv_StringToText` Text))
  (`SceneComponent.K2_SetWorldLocation` _comments (`KismetMathLibrary.MakeVector` _returnvalue_x _returnvalue_y (+ _returnvalue_z 35.0)) false false)
  (`KismetSystemLibrary.RetriggerableDelay` 3.0)
  (`TextRenderComponent.K2_SetText` _comments (`KismetTextLibrary.Conv_StringToText` "")))

(event `InputAction|Attack`
  (params (Key :type "Key Structure" :default "AnyKey"))
  (bind _sprite (`self.Sprite`))
  ;[1 1 1] Shooting
  (:`Pressed`
    (set `self.Character_states` "NewEnumerator6")
    (`self.UpdateAnimation`)
    (`self.DisableInput` null)
    (`KismetSystemLibrary.Delay` (- (`PaperFlipbookComponent.GetFlipbookLength` _sprite) (`PaperFlipbookComponent.GetPlaybackPosition` _sprite)))
    (`PaperFlipbookComponent.SetLooping` (`self.Sprite`) true)
    (set `self.Character_states` "NewEnumerator1")
    (`self.EnableInput` null)))

(event `self.ReceiveTick`
  (params (DeltaSeconds :type "Float (single-precision)"))
  ;[1 1 1] Comment_Event
  (`SceneComponent.K2_SetWorldRotation` (`self.Comments`) (`KismetMathLibrary.MakeRotator` 0.0 0.0 90.0) false false))

(fn `UserConstructionScript`)