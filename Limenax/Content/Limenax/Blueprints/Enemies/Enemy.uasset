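; Enemy Blueprint for a 2D side-view character that uses hare flipbooks and switches animation based on its movement.
; Each tick, horizontal velocity sets the facing yaw, while vertical velocity sets jump and fall flags or selects Running or Standing.
; UpdateAnimation maps the state enum to a flipbook, though nothing here sets the Jumping, Attack or Falling states.
; Landing clears the falling flag and returns the state to Standing.
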(event `self.ReceiveTick`
  (params (DeltaSeconds :type "Float (single-precision)"))
  (bind (_returnvalue_x _returnvalue_y _returnvalue_z) (`KismetMathLibrary.BreakVector` (`self.GetVelocity`)))
  ;[1 1 1] Set state and rotation
  (`|ExecutionSequence`
    (:`then_0`
      (`/Engine/EditorBlueprintResources/StandardMacros.CompareFloat` _returnvalue_x
        (:`>`
          (`self.SetActorRotation` (`KismetMathLibrary.MakeRotator` 0.0)))
        (:`<`
          (`self.SetActorRotation` (`KismetMathLibrary.MakeRotator` 0.0 0.0 180.0))))
      (`self.UpdateAnimation` :!label _label))
    (:`then_1`
      (`/Engine/EditorBlueprintResources/StandardMacros.CompareFloat` 0.0 _returnvalue_z
        (:`>`
          (set `self.isJumping` true))
        (:`==`
          (`/Engine/EditorBlueprintResources/StandardMacros.CompareFloat` _returnvalue_x
            (:`>`
              _)
            (:`==`
              (set `self.Character_states` "NewEnumerator1")
              (goto _label))
            (:`<`
              _))
          (set `self.Character_states` "NewEnumerator0")
          (goto _label))
        (:`<`
          (set `self.isJumping` false)
          (set `self.isFalling` true))))))

(event `self.OnLanded`
  (params (Hit :type "HitResult Structure (by ref)"))
  (set `self.isFalling` false)
  (set `self.Character_states` "NewEnumerator1"))

(event `UpdateAnimation`
  (bind _sprite (`self.Sprite`))
  ;[1 1 1] Update animation
  (switch `/Game/Limenax/Blueprints/Character_states` (`self.Character_states`)
    (:`NewEnumerator0`
      (`PaperFlipbookComponent.SetFlipbook` _sprite "/Game/Limenax/Character/Enemies/Hare/HareMove.HareMove"))
    (:`NewEnumerator1`
      (`PaperFlipbookComponent.SetFlipbook` _sprite "/Game/Limenax/Character/Enemies/Hare/HareStay.HareStay"))
    (:`NewEnumerator2`
      (`PaperFlipbookComponent.SetFlipbook` _sprite "/Game/Limenax/Character/Enemies/Hare/HareJump2.HareJump2"))
    (:`NewEnumerator5`
      (`PaperFlipbookComponent.SetFlipbook` _sprite "/Game/Limenax/Character/Enemies/Hare/HareAttack.HareAttack"))
    (:`NewEnumerator8`
      (`PaperFlipbookComponent.SetFlipbook` _sprite "/Game/Limenax/Character/Enemies/Hare/HareFall.HareFall"))))

(fn `UserConstructionScript`)