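; AI controller for enemies that chase and attack the player within a visible distance and return to their spawn actor otherwise.
; Tick compares X-axis distance to the player, pausing or resuming a looping MoveToPlayer timer.
; MoveToPlayer calls Attack on arrival, while a DoOnce limits MoveToSpawn to one call each time the player leaves range.
; Patrol is empty, and its random back-and-forth movement logic is disconnected.
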(event Custom|MoveToSpawn
  ;[1 1 1] Ai movement
  (bind _asenemy (Utilities|Casting|CastToEnemy (Pawn|GetControlledPawn)))
  (AI|Navigation|SimpleMovetoActor (Pawn|GetController _asenemy) (Variables|/Game/Limenax/Blueprints/Enemies/Enemy.Enemy_C|GetSpawnActor _asenemy)))

(event Custom|Patrol
  ;[1 1 1] Ai movement
)

(event Custom|MoveToPlayer
  (bind _returnvalue (Pawn|GetControlledPawn))
  ;[1 1 1] Ai movement
  (Utilities|Time|PauseTimerbyHandle (Variables|Default|GetPatrolTimer))
  (AI|AIMoveTo _returnvalue "0,0.000000, 0" (Game|GetPlayerCharacter 0) 25.0 false
    (:OnSuccess
      (bind _asenemy (Utilities|Casting|CastToEnemy _returnvalue))
      (Default|Attack _asenemy))))

(event EventBeginPlay
  ;[1 1 1] Initialization
  (bind _returnvalue (Utilities|Time|SetTimerbyFunctionName 0 "MoveToPlayer" 0.1 true))
  (Variables|Default|SetMoveTimer _returnvalue)
  (Utilities|Casting|CastToEnemy (Pawn|GetControlledPawn)))

(event EventTick
  (params (DeltaSeconds :type Float%20%28single-precision%29))
  (bind _movetimer (Variables|Default|GetMoveTimer))
  (bind _dist (CallFunction|GetDistanceBetweenObjects (Game|GetPlayerCharacter 0) (Pawn|GetControlledPawn)))
  (if (<= (.x _dist) (Variables|Default|GetVisibleDistance))
    (Utilities|Time|UnpauseTimerbyHandle _movetimer)
    (goto _label Reset)
    (else
      (Utilities|Time|PauseTimerbyHandle _movetimer)
      (Utilities|FlowControl|DoOnce false :!label _label
        (:Completed
          (CallFunction|MovetoSpawn))))))

(fn ConstructionScript)

(fn GetDistanceBetweenObjects
  (params (Object1 :type Actor%20Object%20Reference) (Object2 :type Actor%20Object%20Reference))
  (bind _returnvalue (Transformation|GetActorLocation Object2))
  (bind _returnvalue_2 (Transformation|GetActorLocation Object1))
  (bind _returnvalue_3 (- _returnvalue_2 _returnvalue))
  (if (or (== Object1 0) (== Object2 0))
    _
    (else
      (Math|Float|CompareFloat (.X (Math|Vector|BreakVector _returnvalue_3)) 0.0
        (:>
          (LocalVariables|SetdistVector _returnvalue_3 :!label _label))
        (:==
          (goto _label))
        (:<
          (LocalVariables|SetdistVector (* _returnvalue_3 -1))))))
  (return (LocalVariables|GetdistVector)))