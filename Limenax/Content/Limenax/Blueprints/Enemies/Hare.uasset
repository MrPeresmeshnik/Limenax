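; Hare enemy Blueprint that supplies its own attack sequence and defers tick, landing and construction to its parent class.
; Attack flags the hare as attacking, halts character movement and switches the animation state.
; After a fixed wind-up delay it calls DamageTransfer if IsHit is set, then changes the animation state again, clears the flag and reactivates movement.
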(event `self.ReceiveBeginPlay`)

(event `self.ReceiveActorBeginOverlap`
  (params (OtherActor :type "Actor Object Reference")))

(event `self.ReceiveTick`
  (params (DeltaSeconds :type "Float (single-precision)"))
  (`parent.ReceiveTick` DeltaSeconds))

(event `self.OnLanded`
  (params (Hit :type "HitResult Structure (by ref)"))
  (`parent.OnLanded` Hit))

(event `self.Attack`
  ;[1 1 1] Attack animation
  (set `self.isAttack` true)
  (`ActorComponent.Deactivate` (`self.CharacterMovement`))
  (set `self.Character_states` "NewEnumerator5")
  (`self.UpdateAnimation`)
  (`KismetSystemLibrary.Delay` 1.34)
  (if (`self.isHit`)
    (`self.DamageTransfer`))
  (`KismetSystemLibrary.Delay` 0.0)
  (set `self.Character_states` "NewEnumerator1")
  (`self.UpdateAnimation`)
  (set `self.isAttack` false)
  (`ActorComponent.Activate` (`self.CharacterMovement`) false))

(fn `UserConstructionScript`
  (`parent.UserConstructionScript`))