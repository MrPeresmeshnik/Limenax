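; Quest enemy spawner that creates a Q1Enemy and sets it moving or attacking.
; CreateEnemy spawns the pawn with its default controller, using the Box's X and Z coordinates and the Arrow's rotation, ignoring collisions.
; If CanMove is set, the enemy waits briefly, then moves to Target1 or Target2 at random.
; Otherwise it attacks immediately.
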(event `CreateEnemy`
  (bind _pawn (`self.Pawn`))
  (bind (_returnvalue_x _returnvalue_y _returnvalue_z) (`KismetMathLibrary.BreakVector` (`SceneComponent.K2_GetComponentLocation` (`self.Box`))))
  (bind _returnvalue (`AIBlueprintHelperLibrary.SpawnAIFromClass` "/Game/Limenax/Blueprints/QuestEnemy/Q1Enemy.Q1Enemy_C" null (`KismetMathLibrary.MakeVector` _returnvalue_x 0.0 _returnvalue_z) (`SceneComponent.K2_GetComponentRotation` (`self.Arrow`)) true))
  (set `self.Pawn` _returnvalue)
  (`Pawn.SpawnDefaultController` _returnvalue)
  (if (`self.canMove`)
    (`KismetSystemLibrary.Delay` 0.5)
    (`/Engine/EditorBlueprintResources/StandardMacros.CompareInt` (mod (`KismetMathLibrary.RandomInteger` 4) 2) 1
      (:`==`
        (bind _asq1enemy (cast `/Game/Limenax/Blueprints/QuestEnemy/Q1Enemy` _pawn))
        (`/Game/Limenax/Blueprints/QuestEnemy/Q1Enemy.MoveToTarget` _asq1enemy (`self.Target1`)))
      (:`<`
        (bind _asq1enemy_2 (cast `/Game/Limenax/Blueprints/QuestEnemy/Q1Enemy` _pawn))
        (`/Game/Limenax/Blueprints/QuestEnemy/Q1Enemy.MoveToTarget` _asq1enemy_2 (`self.Target2`))))
    (else
      (bind _returnvalue_2 (`AIBlueprintHelperLibrary.GetAIController` _returnvalue))
      (bind _asq1enemy_3 (cast `/Game/Limenax/Blueprints/QuestEnemy/Q1Enemy` (`Controller.K2_GetPawn` _returnvalue_2)))
      (`/Game/Limenax/Blueprints/QuestEnemy/Q1Enemy.Attack` _asq1enemy_3))))

(fn `UserConstructionScript`)