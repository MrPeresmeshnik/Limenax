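; Q1Enemy is a flipbook-sprite enemy that moves to a given target, then fires Bullets in an endless loop timed to its animation.
; Tick picks running or standing flipbooks from X velocity and updates an overhead health bar widget.
; Any damage feeds the player's kill bar, but only Bullets not tagged as its own type reduce health.
; Death spawns a Plane_BP, awards experience and destroys it.
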(event `self.ReceiveBeginPlay`
  (bind (_returnvalue_x _returnvalue_y _returnvalue_z) (`KismetMathLibrary.BreakVector` (`SceneComponent.K2_GetComponentLocation` (`self.Sprite`))))
  (`|SpawnActorFromClass` "/Game/Limenax/Mission/Plane_BP.Plane_BP_C" (`KismetMathLibrary.MakeTransform` (`KismetMathLibrary.MakeVector` _returnvalue_x _returnvalue_y (+ _returnvalue_z 10.0))) "Undefined" "OverrideRootScale"))

(event `MoveToTarget`
  (params (TargetActor :type "Actor Object Reference"))
  ;[1 1 1] Move to target
  (`|AIMoveTo` self (`self.K2_GetActorLocation` TargetActor)
    (:`then`
      (`/Engine/EditorBlueprintResources/StandardMacros.DoOnce` false
        (:`Completed`
          (set `self.bUseControllerRotationYaw` false))))
    (:`OnSuccess`
      (`self.Attack`))))

(event `Attack`
  ;[1 1 1] Attack
  (if (not (`self.isAttack`))
    (set `self.Character_states` "NewEnumerator5")
    (set `self.isAttack` true)
    (`self.UpdateAnimation`)
    (`self.Shooting`)))

(event `self.ReceiveAnyDamage`
  (params (Damage :type "Float (single-precision)") (DamageType :type "DamageType Object Reference") (InstigatedBy :type "Controller Object Reference") (DamageCauser :type "Actor Object Reference"))
  ;[1 1 1] Event damage
  (bind _asmain_player (cast `/Game/Limenax/Blueprints/MainPlayer` (`GameplayStatics.GetPlayerCharacter` 0)))
  (`/Game/Limenax/Blueprints/MainPlayer.Kill Bar Event` _asmain_player 25)
  (bind _asbullet (cast `/Game/Limenax/Blueprints/Bullet` DamageCauser))
  (if (not (== (`KismetArrayLibrary.Array_Get` (`Actor.Tags` (`/Game/Limenax/Blueprints/Bullet.Actor` _asbullet))) "q1enemy"))
    (bind _output_get (set `self.Health` (- (`self.Health`) Damage)))
    (if (<= _output_get 0.0)
      (`self.Die`))))

(event `Shooting`
  (bind _sprite (`self.Sprite`))
  (bind _returnvalue (`SceneComponent.K2_GetComponentToWorld` (`self.SpawnBullet`)))
  (`|SpawnActorFromClass` "/Game/Limenax/Blueprints/Bullet.Bullet_C" (`KismetMathLibrary.MakeTransform` (`KismetMathLibrary.MakeVector` (.x (.location _returnvalue)) 0.0 (.z (.location _returnvalue))) (.rotation _returnvalue) (.scale _returnvalue)) "Undefined" "OverrideRootScale" null (`self.Damage`) self)
  (`KismetSystemLibrary.Delay` (- (`PaperFlipbookComponent.GetFlipbookLength` _sprite) (`PaperFlipbookComponent.GetPlaybackPosition` _sprite)))
  (`self.Shooting`))

(event `UpdateAnimation`
  (bind _sprite (`self.Sprite`))
  ;[1 1 1] Update animation
  (switch `/Game/Limenax/Blueprints/Character_states` (`self.Character_states`)
    (:`NewEnumerator0`
      (`PaperFlipbookComponent.SetFlipbook` _sprite "/Game/Limenax/Character/QuestEnemy/q1move.q1move"))
    (:`NewEnumerator1`
      (`PaperFlipbookComponent.SetFlipbook` _sprite "/Game/Limenax/Character/QuestEnemy/q1Stay.q1Stay"))
    (:`NewEnumerator5`
      (`PaperFlipbookComponent.SetFlipbook` _sprite "/Game/Limenax/Character/QuestEnemy/q1Attack.q1Attack"))))

(event `Die`
  (bind (_returnvalue_x _returnvalue_y _returnvalue_z) (`KismetMathLibrary.BreakVector` (`SceneComponent.K2_GetComponentLocation` (`self.Sprite`))))
  (`|SpawnActorFromClass` "/Game/Limenax/Mission/Plane_BP.Plane_BP_C" (`KismetMathLibrary.MakeTransform` (`KismetMathLibrary.MakeVector` _returnvalue_x 0.0 (+ _returnvalue_z 10.0))) "Undefined" "OverrideRootScale" null self)
  (bind _asmain_player (cast `/Game/Limenax/Blueprints/MainPlayer` (`GameplayStatics.GetPlayerCharacter` 0)))
  (`/Game/Limenax/Blueprints/MainPlayer.Experience+` _asmain_player (`self.experience`))
  (`self.K2_DestroyActor`))

(event `self.ReceiveTick`
  (params (DeltaSeconds :type "Float (single-precision)"))
  (bind _returnvalue_x (`KismetMathLibrary.BreakVector` (`self.GetVelocity`)))
  (`|ExecutionSequence`
    (:`then_0`
      ;[1 1 1] Update animation
      (`/Engine/EditorBlueprintResources/StandardMacros.CompareFloat` _returnvalue_x
        (:`>`
          (set `self.Character_states` "NewEnumerator0")
          (`self.UpdateAnimation` :!label _label))
        (:`==`
          (if (not (`self.isAttack`))
            (set `self.Character_states` "NewEnumerator1")
            (goto _label)))))
    (:`then_1`
      (`SceneComponent.K2_SetWorldRotation` (`self.Widget`) (struct :`Yaw` 90.0) false false))
    (:`then_2`
      (bind _asq_1enemy_widget (cast `/Game/Limenax/interface/q1enemy/q1enemy_widget` (`WidgetComponent.GetUserWidgetObject` (`self.Widget`))))
      (`ProgressBar.SetPercent` (`/Game/Limenax/interface/q1enemy/q1enemy_widget.ProgressBar_273` _asq_1enemy_widget) (/ (`self.Health`) (`self.FullHealth`))))))

(fn `UserConstructionScript`)