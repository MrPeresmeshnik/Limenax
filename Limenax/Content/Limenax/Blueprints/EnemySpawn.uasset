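; EnemySpawn is a spawner actor that keeps the level stocked with Enemy AI pawns up to MaxNumberEnemy.
; A fast looping timer calls Spawn, which counts all Enemy actors and, below the cap, spawns one at the Box location with a random X offset.
; Each new pawn gets a default controller and stores a reference back to this spawner in SpawnActor.
; An older DoOnce/Delay spawn chain remains in the graph but never runs.
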(event `self.ReceiveBeginPlay`
  (`KismetSystemLibrary.K2_SetTimer` null "Spawn" 0.2 true))

(event `Spawn`
  (bind _enemy (`self.Enemy`))
  (bind _outactors (`GameplayStatics.GetAllActorsOfClass` _enemy))
  (if (<= (`KismetArrayLibrary.Array_Length` _outactors) (- (`self.MaxNumberEnemy`) 1))
    (bind _returnvalue (`AIBlueprintHelperLibrary.SpawnAIFromClass` _enemy null (+ (`SceneComponent.K2_GetComponentLocation` (`self.Box`)) (`KismetMathLibrary.MakeVector` (`KismetMathLibrary.Conv_IntToDouble` (`KismetMathLibrary.RandomInteger` 500)))) (struct)))
    (`Pawn.SpawnDefaultController` _returnvalue)
    (bind _returnvalue_2 (`AIBlueprintHelperLibrary.GetAIController` _returnvalue))
    (bind _asenemy (cast `/Game/Limenax/Blueprints/Enemies/Enemy` (`Controller.K2_GetPawn` _returnvalue_2)))
    (set `/Game/Limenax/Blueprints/Enemies/Enemy.SpawnActor` self _asenemy)))

(event `self.ReceiveTick`
  (params (DeltaSeconds :type "Float (single-precision)")))

(fn `UserConstructionScript`)